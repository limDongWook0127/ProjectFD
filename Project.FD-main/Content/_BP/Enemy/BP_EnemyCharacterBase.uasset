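; Base enemy character Blueprint that sets up the enemy's health bar name and handles cleanup on death.
; On BeginPlay, it passes EnemyName to the WBP_EnemyHealthBar held in its widget component.
; OnEnemyDie deactivates the Shared.Ability.Death ability through the ability system component, then destroys directly attached actors and the enemy itself.
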(event EventBeginPlay
  (CallFunction|ChangeName))

(event EventOnEnemyDie
  (Class|BaseAbilitySystemComponent|TryDeactivateAbilitybyTag (Variables|Default|GetBaseAbilitySystemComponent) "(TagName=\"Shared.Ability.Death\")")
  (bind _output_get (Variables|Default|SetOut%20Actors (Actor|GetAttachedActors false false)))
  (for _array_element _output_get
    (Actor|DestroyActor _array_element))
  (Actor|DestroyActor))

(fn ConstructionScript)

(fn ChangeName
  (bind _aswbp_enemy_health_bar (Utilities|Casting|CastToWBP_EnemyHealthBar (UserInterface|GetWidget (Variables|Default|GetWidgetComponent))))
  (Default|ChangeName _aswbp_enemy_health_bar (Utilities|Text|ToText(String) (Variables|Default|GetEnemyName))))