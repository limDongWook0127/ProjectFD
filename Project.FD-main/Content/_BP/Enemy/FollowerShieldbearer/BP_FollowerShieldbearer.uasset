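; BP_FollowerShieldbearer is an enemy Blueprint for a follower shieldbearer that removes its attached shield when destroyed.
; On BeginPlay it runs the parent logic and binds DestroyShield to its OnDestroyed event.
; DestroyShield destroys every directly attached actor, without checking type or recursing into nested attachments.
; Overlap and Tick events are disabled, and the construction script only calls the parent.
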(event Custom|DestroyShield
  (params (DestroyedActor :type Actor%20Object%20Reference))
  ;[1 1 1] Comment
  (for _array_element (Actor|GetAttachedActors DestroyedActor false false)
    (Actor|DestroyActor _array_element)))

(event EventBeginPlay
  (|CallParentFunction)
  ;[1 1 1] Comment
  (Game|BindEventtoOnDestroyed (delegate Custom|DestroyShield)))

(event Collision|EventActorBeginOverlap
  (params (OtherActor :type Actor%20Object%20Reference))
  (|CallParentFunction OtherActor) ; This node is disabled and will not be called.\nDrag off pins to build functionality.
)

(event EventTick
  (params (DeltaSeconds :type Float%20%28single-precision%29))
  (|CallParentFunction DeltaSeconds) ; This node is disabled and will not be called.\nDrag off pins to build functionality.
)

(fn ConstructionScript
  (|CallParentFunction))