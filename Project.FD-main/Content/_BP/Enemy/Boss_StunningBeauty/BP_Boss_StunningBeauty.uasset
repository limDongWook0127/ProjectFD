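; Boss enemy Blueprint for the Stunning Beauty boss, extending a parent class with its spawn animation and player tracking.
; BeginPlay runs the parent logic, caches the player character and plays the spawn montage.
; Tick stores the look-at pitch from the left upper-arm socket to the player in PlayerSeePitch.
; ChangeName passes EnemyName to the boss health widget.
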(event EventBeginPlay
  (bind _returnvalue (Game|GetPlayerCharacter 0))
  (|CallParentFunction)
  (Utilities|FlowControl|Sequence
    (:then_0
      (Utilities|IsValid _returnvalue
        (:Is%20Valid
          (Variables|Default|SetPlayerCharacter _returnvalue))))
    (:then_1
      (Animation|PlayAnimMontage "/Game/_BP/Enemy/Boss_StunningBeauty/Animation/Montage/Spawn_Montage.Spawn_Montage" 1.0 "None"))))

(event Collision|EventActorBeginOverlap
  (params (OtherActor :type Actor%20Object%20Reference))
  (|CallParentFunction OtherActor) ; This node is disabled and will not be called.\nDrag off pins to build functionality.
)

(event EventTick
  (params (DeltaSeconds :type Float%20%28single-precision%29))
  (Variables|Default|SetPlayerSeePitch (.pitch (Math|Rotator|FindLookatRotation (Transformation|GetSocketLocation (Variables|Character|GetMesh self) "Bip001-L-UpperArm") (Transformation|GetActorLocation (Variables|Default|GetPlayerCharacter))))))

(fn ConstructionScript
  (|CallParentFunction))

(fn ChangeName
  (Default|ChangeName (Variables|Default|GetBossHealthWidget) (Utilities|Text|ToText(String) (Variables|Default|GetEnemyName))))