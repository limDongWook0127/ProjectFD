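; BP_Promenade is a Stunning Beauty boss projectile that flies a randomized curved path to the player's location captured at BeginPlay.
; After a short delay it picks a random point toward the target, offsets it by random radius and angle, and activates Niagara.
; A gated Tick interpolates this control point toward the target while the actor chases it at the same speed, bending the path without a spline.
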(event EventBeginPlay
  (|CallParentFunction)
  (Variables|Default|SetTargetLocation (Transformation|GetActorLocation (Game|GetPlayerCharacter 0)))
  (Utilities|FlowControl|Delay 0.01)
  (CallFunction|MidPointCalculator)
  (CallFunction|CurveControlPoint)
  (Components|Activation|Activate (Variables|Default|GetNiagaraComponent) false)
  (Utilities|FlowControl|Gate true) ; enters at Open
)

(event Collision|EventActorBeginOverlap
  (params (OtherActor :type Actor%20Object%20Reference)))

(event EventTick
  (params (DeltaSeconds :type Float%20%28single-precision%29))
  (Utilities|FlowControl|Gate true
    (:Exit
      (if true
        (if (Utilities|Operators|NotEqual(!=) (Transformation|GetActorLocation) (Variables|Default|GetTargetLocation) 0.0)
          (Variables|Default|SetCurvedPoint (Math|Interpolation|VInterptoConstant (Variables|Default|GetCurvedPoint) (Variables|Default|GetTargetLocation) (Utilities|Time|GetWorldDeltaSeconds) (Variables|Default|GetProjectile%20Speed)))
          (Transformation|SetActorLocation (Math|Interpolation|VInterptoConstant (Transformation|GetActorLocation) (Variables|Default|GetCurvedPoint) (Utilities|Time|GetWorldDeltaSeconds) (Variables|Default|GetProjectile%20Speed)) false false))))))

(fn ConstructionScript
  (|CallParentFunction))

(fn MidPointCalculator
  (Variables|Default|SetMidPoint (+ (* (- (Variables|Default|GetTargetLocation) (Transformation|GetActorLocation)) (Math|Random|RandomFloatinRange (Variables|Default|GetMinCurvePointDistance) (Variables|Default|GetMaxCurvePointDistance))) (Transformation|GetActorLocation))))

(fn CurveControlPoint
  (bind _midpoint (Variables|Default|GetMidPoint))
  (bind _targetlocation (Variables|Default|GetTargetLocation))
  (bind _returnvalue (Math|Rotator|FindLookatRotation _midpoint _targetlocation))
  (bind (_x _y) (Math|Rotator|BreakRotIntoAxes _returnvalue))
  (Variables|Default|SetCurvedPoint (+ (Variables|Default|GetMidPoint) (Math|Vector|RotateVectorAroundAxis (* (Math|Random|RandomFloatinRange (Variables|Default|GetMinCurveRadius) (Variables|Default|GetMaxCurveRadius)) _y) (Math|Random|RandomFloatinRange (Variables|Default|GetMinAngle) (Variables|Default|GetMaxAngle)) _x))))