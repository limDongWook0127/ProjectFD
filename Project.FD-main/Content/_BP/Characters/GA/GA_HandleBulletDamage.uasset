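; GA_HandleBulletDamage is a hero gameplay ability that applies bullet damage to hit targets.
; It waits for bullet hit gameplay events, then builds a GE_DealDamage spec from the equipped AR's damage, or the DMR's otherwise, scaled down by a fixed divisor.
; On successful application it sends a hit react event to the target.
; Each hit also calls HitEvent on the BP_Bunny hero.
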(event Ability|EventActivateAbility
  (bind _payload (Ability|Tasks|WaitGameplayEvent "(TagName=\"Player.Event.Hit.Bullet\")" 0)
    (:EventReceived
      (CallFunction|HandleApplyDamage _payload)
      (Default|HitEvent (.AsBP%20Bunny (Utilities|Casting|CastToBP_Bunny (Class|HeroGameplayAbility|GetHeroCharacterfromActorInfo)))))))

(event Ability|EventOnEndAbility
  (params (bWasCancelled :type Boolean)))

(fn HandleApplyDamage
  (params (GameplayEventData :type Gameplay%20Event%20Data%20Structure%20%28by%20ref%29))
  (bind _returnvalue (Class|HeroGameplayAbility|GetHeroCharacterfromActorInfo))
  (bind _inventorycomponent (Variables|/Script/ProjectA.HeroCharacter|GetInventoryComponent _returnvalue))
  (bind _output_get (LocalVariables|SetNewLocalVar (.Target (Utilities|Struct|BreakGameplayEventData GameplayEventData))))
  (Class|BaseGameplayAbility|ApplyEffectSpecHandletoTarget _output_get (Class|HeroGameplayAbility|MakeHeroDamageEffectSpecHandle "/Game/_BP/Shared/GE/GE_DealDamage.GE_DealDamage_C" (/ (select (== (Variables|/Script/ProjectA.PawnCombatComponent|GetCurrentEquippedWeaponTag (Class|HeroGameplayAbility|GetHeroCombatComponentfromActorInfo)) "(TagName=\"Player.Weapon.AR\")") (.Damage (Utilities|Struct|BreakItemInfo_ (Class|InventoryComponent|GetEquipAR _inventorycomponent))) (.Damage (Utilities|Struct|BreakItemInfo_ (Class|InventoryComponent|GetEquipDMR _inventorycomponent)))) 2e+02) "(TagName=\"Player.SetBycaller.AttackType.Bullet\")")
    (:Success
      (Ability|SendGameplayEventtoActor (LocalVariables|GetNewLocalVar) "(TagName=\"shared.Event.HitReact\")" GameplayEventData))))