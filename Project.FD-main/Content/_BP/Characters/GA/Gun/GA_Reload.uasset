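; Gameplay ability that reloads the Bunny hero's equipped AR or DMR.
; It ends at once if the inventory's max bullet count for that weapon is zero; otherwise it plays one lower-body AR reload montage for both weapons, with an occasional random voice line.
; On montage blend-out, BulletComponent attempts the refill for the equipped weapon tag and the ability ends; interruption ends it without refilling.
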(event Ability|EventActivateAbility
  (bind _asbp_bunny (Utilities|Casting|CastToBP_Bunny (Ability|GetAvatarActorfromActorInfo)))
  (if (!= (Math|Integer|SelectInt (Class|InventoryComponent|GetMaxBulletAR (Variables|/Script/ProjectA.HeroCharacter|GetInventoryComponent _asbp_bunny)) (Class|InventoryComponent|GetMaxBulletDMR (Variables|/Script/ProjectA.HeroCharacter|GetInventoryComponent _asbp_bunny)) (== (Variables|/Script/ProjectA.PawnCombatComponent|GetCurrentEquippedWeaponTag (Variables|/Script/ProjectA.HeroCharacter|GetHeroCombatComponent _asbp_bunny)) "(TagName=\"Player.Weapon.AR\")")) 0)
    (Animation|Montage|PlayMontage (Variables|/Script/Engine.Character|GetMesh _asbp_bunny) "/Game/Assets/Bunny/Animation/Montages/AM_F_2LT_AR_1007_Reload_Lower.AM_F_2LT_AR_1007_Reload_Lower"
      (:then
        (if (>= (Math|Random|RandomFloatinRange 0.0 1e+02) 7e+01)
          (Audio|PlaySound2D "/Game/Assets/Bunny/Sound/Voice/Bunny_Vo_Reload_Word_02_wem.Bunny_Vo_Reload_Word_02_wem" 1.0 1.0 0.0 0 0)))
      (:OnBlendOut
        (if (== (Variables|/Script/ProjectA.PawnCombatComponent|GetCurrentEquippedWeaponTag (Variables|/Script/ProjectA.HeroCharacter|GetHeroCombatComponent _asbp_bunny)) "(TagName=\"Player.Weapon.AR\")")
          (Class|BulletSystemComponent|TryReloadBulletAR (Variables|/Script/ProjectA.HeroCharacter|GetBullet_Component _asbp_bunny))
          (else
            (Class|BulletSystemComponent|TryReloadBulletDMR (Variables|/Script/ProjectA.HeroCharacter|GetBullet_Component _asbp_bunny))))
        (Ability|EndAbility :!label _label))
      (:OnInterrupted
        (goto _label)))
    (else
      (Ability|EndAbility))))