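; GA_GainMp is a passive gameplay ability that regenerates the avatar's mana over time.
; On activation it starts a fast looping timer that compares two float attributes on the avatar, presumably current and maximum mana.
; While the first is lower, each tick applies the GE_UseMana effect with a negative cost, reusing the spend effect to restore mana.
; Ending the ability clears the timer.
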(event Custom|GainMana
  (bind _returnvalue (Ability|GetAvatarActorfromActorInfo))
  (bind (_bsuccessfullyfoundattribute _returnvalue_2) (Ability|Attribute|GetFloatAttribute _returnvalue "(AttributeName=\"MaxMp\",Attribute=/Script/ProjectA.BaseAttributeSet:MaxMp,AttributeOwner=\"/Script/CoreUObject.Class'/Script/ProjectA.BaseAttributeSet'\")"))
  (bind (_bsuccessfullyfoundattribute_2 _returnvalue_3) (Ability|Attribute|GetFloatAttribute _returnvalue "(AttributeName=\"CurrentMp\",Attribute=/Script/ProjectA.BaseAttributeSet:CurrentMp,AttributeOwner=\"/Script/CoreUObject.Class'/Script/ProjectA.BaseAttributeSet'\")"))
  (if (Math|Boolean|ANDBoolean _bsuccessfullyfoundattribute_2 _bsuccessfullyfoundattribute (< _returnvalue_3 _returnvalue_2))
    (Class|BaseGameplayAbility|ApplyEffectSpecHandletoTarget (Ability|GetAvatarActorfromActorInfo) (Class|HeroGameplayAbility|MakeHeroUsingManaEffectSpecHandle "/Game/Assets/Bunny/GE/GE_UseMana.GE_UseMana_C" -0.2))))

(event Ability|EventActivateAbility
  (bind _returnvalue (Utilities|Time|SetTimerbyEvent (delegate Custom|GainMana) 0.05 true true))
  (Variables|Default|SetTimerHandle _returnvalue))

(event Ability|EventOnEndAbility
  (params (bWasCancelled :type Boolean))
  (Utilities|Time|ClearandInvalidateTimerbyHandle (Variables|Default|GetTimerHandle)))