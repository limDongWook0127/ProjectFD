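; Passive gameplay ability that adjusts a hero's passive resource based on movement speed, apparently building it up as the hero moves.
; On activation, a fast looping timer applies GE_UsePassive to the avatar, passing its velocity length times a small negative factor as the usage amount, so negative use acts as gain.
; The timer is cleared when the ability ends.
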(event Custom|GainPassive
  (bind _returnvalue (Ability|GetAvatarActorfromActorInfo))
  (Class|BaseGameplayAbility|ApplyEffectSpecHandletoTarget _returnvalue (Class|HeroGameplayAbility|MakeHeroUsingPassiveEffectSpecHandle "/Game/Assets/Bunny/GE/GE_UsePassive.GE_UsePassive_C" (* (Math|Vector|VectorLength (Transformation|GetVelocity _returnvalue)) -0.0005))))

(event Ability|EventActivateAbility
  (bind _returnvalue (Utilities|Time|SetTimerbyEvent (delegate Custom|GainPassive) 0.05 true true))
  (Variables|Default|SetTimerHandle _returnvalue))

(event Ability|EventOnEndAbility
  (params (bWasCancelled :type Boolean))
  (Utilities|Time|ClearandInvalidateTimerbyHandle (Variables|Default|GetTimerHandle)))