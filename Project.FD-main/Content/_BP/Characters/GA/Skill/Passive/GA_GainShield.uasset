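; GA_GainShield is a passive gameplay ability that gradually adds shield to the avatar actor while active.
; On activation it starts a fast looping timer that compares two float attributes on the avatar, presumably current and maximum shield.
; While the first is lower, each tick applies a GE_GainShield effect spec carrying a small fixed gain.
; Ending the ability clears the timer.
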(event Custom|GainShield
  (bind _returnvalue (Ability|GetAvatarActorfromActorInfo))
  (bind (_bsuccessfullyfoundattribute _returnvalue_2) (Ability|Attribute|GetFloatAttribute _returnvalue "(AttributeName=\"MaxShield\",Attribute=/Script/ProjectA.HeroAttributeSet:MaxShield,AttributeOwner=\"/Script/CoreUObject.Class'/Script/ProjectA.HeroAttributeSet'\")"))
  (bind (_bsuccessfullyfoundattribute_2 _returnvalue_3) (Ability|Attribute|GetFloatAttribute _returnvalue "(AttributeName=\"CurrentShield\",Attribute=/Script/ProjectA.HeroAttributeSet:CurrentShield,AttributeOwner=\"/Script/CoreUObject.Class'/Script/ProjectA.HeroAttributeSet'\")"))
  (if (Math|Boolean|ANDBoolean _bsuccessfullyfoundattribute_2 _bsuccessfullyfoundattribute (< _returnvalue_3 _returnvalue_2))
    (Class|BaseGameplayAbility|ApplyEffectSpecHandletoTarget (Ability|GetAvatarActorfromActorInfo) (Class|HeroGameplayAbility|MakeHeroGainingShieldEffectSpecHandle "/Game/Assets/Bunny/GE/GE_GainShield.GE_GainShield_C" 0.1))))

(event Ability|EventActivateAbility
  (bind _returnvalue (Utilities|Time|SetTimerbyEvent (delegate Custom|GainShield) 0.1 true true))
  (Variables|Default|SetTimerHandle _returnvalue))

(event Ability|EventOnEndAbility
  (params (bWasCancelled :type Boolean))
  (Utilities|Time|ClearandInvalidateTimerbyHandle (Variables|Default|GetTimerHandle)))