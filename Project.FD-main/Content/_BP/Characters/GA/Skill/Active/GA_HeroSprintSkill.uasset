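; Gameplay Ability for BP_Bunny's sprint skill, a fast dash sustained by mana.
; Activation ends immediately if zoomed in; otherwise it commits cooldown, drops the shoot pose, raises walk speed and starts looping audio and toe sparks.
; A looping timer calls TryUseMana; on failure it restores the cached speed, clears effects and ends the ability.
; The file shows no other cleanup path.
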(event Custom|Sprinting
  (bind _s_ok (CallFunction|TryUseMana))
  (if (not _s_ok)
    (Utilities|Time|ClearandInvalidateTimerbyHandle (Variables|Default|GetTimerHandler))
    (Audio|Components|Audio|Stop (Variables|Default|GetPC_Se_Bunny_Active2_Dash_Loop_wem))
    (Audio|PlaySound2D "/Game/Assets/Bunny/Sound/Skill/PC_Se_Bunny_Active2_DeActive_wem.PC_Se_Bunny_Active2_DeActive_wem" 1.0 1.0 0.0 0 0)
    (Variables|/Script/Engine.CharacterMovementComponent|SetMaxWalkSpeed (Variables|Default|GetCharacter%20Movement) (Variables|Default|GetCachedWalkSpeed))
    (Components|DestroyComponent (Variables|Default|GetRightFx))
    (Components|DestroyComponent (Variables|Default|GetLeftFx))
    (Ability|EndAbility)))

(event Ability|EventActivateAbility
  (bind _asbp_bunny (Utilities|Casting|CastToBP_Bunny (Ability|GetAvatarActorfromActorInfo)))
  (if (Variables|/Game/Assets/Bunny/BP_Bunny.BP_Bunny_C|GetZoomedIn _asbp_bunny)
    (Ability|EndAbility)
    (else
      (Ability|CommitAbilityCooldown false)
      (Audio|PlaySound2D "/Game/Assets/Bunny/Sound/Voice/SC_Skill2.SC_Skill2" 1.0 1.0 0.0 0 0)
      (Default|UnSetShootPose _asbp_bunny)
      (Variables|Default|SetCachedWalkSpeed (Variables|/Script/Engine.CharacterMovementComponent|GetMaxWalkSpeed (Variables|/Script/Engine.Character|GetCharacterMovement _asbp_bunny)))
      (Variables|/Script/Engine.CharacterMovementComponent|SetMaxWalkSpeed (Variables|/Script/Engine.Character|GetCharacterMovement _asbp_bunny) 1.2e+03)
      (Variables|Default|SetCharacter%20Movement (Variables|/Script/Engine.Character|GetCharacterMovement _asbp_bunny))
      (Audio|PlaySound2D "/Game/Assets/Bunny/Sound/Skill/PC_Se_Bunny_Active2_Dash_Start_wem.PC_Se_Bunny_Active2_Dash_Start_wem" 1.0 1.0 0.0 0 0)
      (bind _returnvalue (Audio|CreateSound2D "/Game/Assets/Bunny/Sound/Skill/PC_Se_Bunny_Active2_Dash_Loop_wem.PC_Se_Bunny_Active2_Dash_Loop_wem" 1.0 1.0 0.0 0))
      (bind _output_get (Variables|Default|SetPC_Se_Bunny_Active2_Dash_Loop_wem _returnvalue))
      (Audio|Components|Audio|Play _output_get 0.0)
      (bind _returnvalue_2 (Effects|SpawnEmitterAttached "/Game/Assets/Bunny/Niagara/Arcs_and_Sparks/Systems/Sparks/Constant/PS_Sparks_Omni_PosX_Constant.PS_Sparks_Omni_PosX_Constant" (Variables|/Script/Engine.Character|GetMesh _asbp_bunny) "Bip001-R-Toe0"))
      (Variables|Default|SetRightFx _returnvalue_2)
      (bind _returnvalue_3 (Effects|SpawnEmitterAttached "/Game/Assets/Bunny/Niagara/Arcs_and_Sparks/Systems/Sparks/Constant/PS_Sparks_Omni_PosX_Constant.PS_Sparks_Omni_PosX_Constant" (Variables|/Script/Engine.Character|GetMesh _asbp_bunny) "Bip001-L-Toe0"))
      (Variables|Default|SetLeftFx _returnvalue_3)
      (bind _returnvalue_4 (Utilities|Time|SetTimerbyEvent (delegate Custom|Sprinting) 0.05 true))
      (Variables|Default|SetTimerHandler _returnvalue_4))))